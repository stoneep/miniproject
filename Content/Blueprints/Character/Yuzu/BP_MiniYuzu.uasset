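; BP_MiniYuzu is a Yuzu character Blueprint that sets up its camera on BeginPlay and supports motion-warped facing.
; UpdateCamera sets the camera field of view, applies a zero world offset and, if enabled, finds the main BP_CameraTrack, assigns itself as owner and makes it the view target.
; SetFacingTarget feeds a location to the MotionWarping "FacingTarget" warp target.
; Tick, facing update and movement-state functions are empty stubs.
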(event Custom|SetFacingTarget
  (params (FacingTarget :type Vector))
  (Class|MotionWarpingComponent|AddorUpdateWarpTargetfromLocation (Variables|Default|GetMotionWarping) "FacingTarget" FacingTarget))

(event EventBeginPlay
  (CallFunction|UpdateCamera))

(event Collision|EventActorBeginOverlap
  (params (OtherActor :type Actor%20Object%20Reference)))

(event EventTick
  (params (DeltaSeconds :type Float%20%28single-precision%29)))

(event EventUpdateFacingTarget
  (params (Target :type Vector%20%28by%20ref%29 :default "0, 0, 0")))

(fn ConstructionScript)

(fn UseMainCameraTrack
  (bind _outactors (Actor|GetAllActorsOfClass "/Game/Camera/BP_CameraTrack.BP_CameraTrack_C"))
  (if (Utilities|Array|IsNotEmpty _outactors)
    (bind _array_element (Utilities|Array|ForEachLoopwithBreak _outactors :!label _label)
      (:LoopBody
        (if (Variables|/Game/Camera/BP_CameraTrack.BP_CameraTrack_C|GetbIsMainTrack? _array_element)
          (bind _output_get (Variables|Default|SetCameraTrack _array_element))
          (Default|SetCamOwner _output_get self)
          (Game|Player|SetViewTargetwithBlend (Game|GetPlayerController 0) (Variables|Default|GetCameraTrack) 0.0 "VTBlend_Linear" 0.0 false)
          (goto _label Break))))))

(fn UpdateEmovementState)

(fn UpdateCamera
  (Camera|SetFieldOfView (Variables|Default|GetCamera) 0.0)
  (Transformation|AddActorWorldOffset "0, 0, 0")
  (if (Variables|Default|GetbUseMainCamTrack?)
    (CallFunction|UseMainCameraTrack)))