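; GA_Bullet is a Gameplay Ability that makes MiniYuzu fire a projectile at the point under the mouse.
; After committing, it takes the hit location from a target-data task and turns the avatar to face it.
; It plays the attack montage and spawns the projectile at the tagged socket when the montage's fire gameplay event arrives.
; The ability ends when the montage completes, blends out, is interrupted or is cancelled.
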(event Ability|EventActivateAbility
  (Ability|CommitAbility)
  (bind _datahandle (|TargetDataUnderMouse)
    (:then
      (Variables|Default|SetProjectileTargetLocation (.Location (Collision|BreakHitResult (Ability|TargetData|GetHitResultfromTargetData _datahandle))))
      (bind _asbp_mini_yuzu (Utilities|Casting|CastToBP_MiniYuzu (Ability|GetAvatarActorfromActorInfo)))
      (Default|SetFacingTarget _asbp_mini_yuzu (Variables|Default|GetProjectileTargetLocation))
      (|PlayMontageandWaitProxy "None" "/Game/Characters/Yuzu/Yuzu_Attack_mtg.Yuzu_Attack_mtg" 1.0 "None" false 1.0 0.0
        (:then
          (Ability|Tasks|WaitGameplayEvent "(TagName=\"Event.Montage.Fire\")" 0
            (:EventReceived
              (Class|MiniProjectileSkill|SpawnProjectile (Variables|Default|GetProjectileTargetLocation) (Variables|Default|GetSocket%20Tag) false 0.0))))
        (:OnCompleted
          (Ability|EndAbility :!label _label))
        (:OnBlendOut
          (goto _label))
        (:OnInterrupted
          (goto _label))
        (:OnCancelled
          (goto _label))))))