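; Enemy ranged attack gameplay ability, so far covering facing, montage playback and socket lookup, with no projectile spawn.
; On activation it turns the avatar toward its combat target through interface messages, then plays a random tagged attack montage.
; It waits for the gameplay event matching that montage's tag, then fetches the combat socket location for the tag.
; That location is not yet used, and the ability never calls EndAbility.
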(event Ability|EventActivateAbility
  (bind _returnvalue (Ability|GetAvatarActorfromActorInfo))
  (bind _returnvalue_2 (Class|EnemyInterface|GetCombatTarget(Message) _returnvalue))
  (Class|CombatInterface|UpdateFacingTarget(Message) _returnvalue (Transformation|GetActorLocation _returnvalue_2))
  (bind _returnvalue_3 (Class|CombatInterface|GetAttackMontages(Message) _returnvalue))
  (bind _output_get (Variables|Default|SetTaggedMontage (Class|MiniDamageGameplayAbility|GetRandomTaggedMontagefromArray _returnvalue_3)))
  (|PlayMontageandWaitProxy "None" (.Montage (Utilities|Struct|BreakTaggedMontage _output_get)) 1.0 "None" false 1.0 0.0
    (:then
      (Ability|Tasks|WaitGameplayEvent (.MontageTag (Utilities|Struct|BreakTaggedMontage _output_get)) 0
        (:EventReceived
          (Class|CombatInterface|GetCombatSocketLocation(Message) (Ability|GetAvatarActorfromActorInfo) (.MontageTag (Utilities|Struct|BreakTaggedMontage _output_get))))))))

(event Ability|EventOnEndAbility
  (params (bWasCancelled :type Boolean)))