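; Enemy gameplay ability that summons random minions at a set of spawn locations.
; On activation it shuffles the locations from GetSpawnLocations and plays a Niagara ground-summon effect at all of them at once.
; After a short delay, a delay-driven loop spawns one minion with its default controller per location, pausing between spawns.
; Spawn height offset is hardcoded, a debug sphere marks each spawn, and EndAbility is never called here.
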(event Ability|EventActivateAbility
  (bind _returnvalue (Class|MiniSummonAbility|GetSpawnLocations))
  (bind _output_get (Variables|Default|SetSpawnLocaion _returnvalue))
  (Utilities|Array|Shuffle _output_get)
  (for _array_element _output_get
    (Niagara|SpawnSystematLocation "/Game/Assets/Effects/Combat/NS_GroundSummon.NS_GroundSummon" _array_element))
  (Utilities|FlowControl|Delay 0.75)
  (if (< (Variables|Default|GetSpawnLocaionIndex) (Utilities|Array|Length (Variables|Default|GetSpawnLocaion))) :!label _label
    (bind _returnvalue_2 (Game|SpawnActorfromClass (Class|MiniSummonAbility|GetRandomMinionClass) (Math|Transform|MakeTransform (+ (Utilities|Array|Get(acopy) (Variables|Default|GetSpawnLocaion) (Variables|Default|GetSpawnLocaionIndex)) "0.000000,0.000000,70.000000") "0, 0, 0" "1.000000,1.000000,1.000000") "AlwaysSpawn" "MultiplyWithRoot" 0 0))
    (Pawn|SpawnDefaultController _returnvalue_2)
    (Rendering|Debug|DrawDebugSphere (Utilities|Array|Get(acopy) (Variables|Default|GetSpawnLocaion) (Variables|Default|GetSpawnLocaionIndex)) 1e+02 12 "(R=1.000000,G=1.000000,B=1.000000,A=1.000000)" 0.0)
    (Math|Integer|IncrementInt (Variables|Default|GetSpawnLocaionIndex)
      (:%20%20
        (Utilities|FlowControl|Delay 1e+01)
        (goto _label)))))