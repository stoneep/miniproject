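; Spline-track camera that follows an owner character, enabling its tick only while a valid owner is set.
; It finds the spine socket's nearest point on Path, steps back by a lag distance and samples CameraTrack at that time for the eased camera location.
; The lag eases larger when the owner moves fast against the path direction.
; Look-at rotation is applied only when the owner is set; rotation smoothing is unwired.
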(event EventTick
  (params (DeltaSeconds :type Float%20%28single-precision%29))
  (bind _cameraowner (Variables|Default|GetCameraOwner)
    (:then
      (CallFunction|UpdateCamera (Transformation|GetSocketLocation (Variables|/Script/Engine.Character|GetMesh _cameraowner) "Bip001-Spine"))
      (CallFunction|InterpLocation)
      (CallFunction|UpdateMovementLagOffset))
    (:else)))

(fn ConstructionScript)

(fn SetCamOwner
  (params (NewParam :type BP%20Mini%20Yuzu%20Object%20Reference))
  (bind _output_get (Variables|Default|SetCameraOwner NewParam))
  (Utilities|IsValid _output_get
    (:Is%20Valid
      (Actor|Tick|SetActorTickEnabled true)
      (CallFunction|UpdateCamera (Transformation|GetSocketLocation (Variables|/Script/Engine.Character|GetMesh (Variables|Default|GetCameraOwner)) "Bip001-Spine"))
      (Transformation|SetWorldLocationAndRotation (Variables|Default|GetCamera) (Variables|Movement|GetDesiredLocation) (Variables|Default|GetDesiredRotation) false true))
    (:Is%20Not%20Valid
      (Actor|Tick|SetActorTickEnabled false))))

(fn UpdateCamera
  (params (WorldLocation :type Vector))
  (Variables|Movement|SetDesiredLocation (Spline|GetLocationatTime (Variables|Default|GetCameraTrack) (CallFunction|GetTimeAlongSplineatNearbyLocation WorldLocation (Variables|Movement|GetMovementLagOffset)) "World" false))
  (Variables|Default|SetDesiredRotation (Math|Rotator|FindLookatRotation (Transformation|GetWorldLocation (Variables|Default|GetCamera)) (Transformation|GetActorLocation (Variables|Default|GetCameraOwner)))))

(fn GetTimeAlongSplineatNearbyLocation
  (params (WorldLocatoin :type Vector) (DistanceLag :type Float%20%28double-precision%29))
  (bind _path (Variables|Default|GetPath))
  (bind _cameraowner (Variables|Default|GetCameraOwner))
  (bind _returnvalue (Class|SplineComponent|FindInputKeyClosesttoWorldLocation _path WorldLocatoin))
  (bind _returnvalue_2 (Transformation|GetVelocity _cameraowner))
  (bind (_x _y) (Math|Vector|BreakVector _returnvalue_2))
  (Variables|Movement|SetLagDirection (Math|Integer|SelectInt (Math|Integer|SelectInt 1 2 (Utilities|Operators|EqualEqual (Math|Rotator|GetRotationXVector (Class|SplineComponent|GetRotationatSplineInputKey (Variables|Default|GetPath) _returnvalue "World")) (Math|Vector|Normalize _returnvalue_2) 1.0)) 0 (> (Math|Vector|VectorLength (Math|Vector|MakeVector _x _y 0.0)) 3e+02)))
  (return (Class|SplineComponent|GetTimeatDistanceAlongSpline (Variables|Default|GetPath) (- (Class|SplineComponent|GetDistanceAlongSplineatSplineInputKey (Variables|Default|GetPath) _returnvalue) DistanceLag))))

(fn InterpLocation
  (bind _camera (Variables|Default|GetCamera))
  (bind _returnvalue (Transformation|GetWorldLocation _camera))
  (if (not (Utilities|Operators|EqualEqual (Variables|Movement|GetDesiredLocation) _returnvalue 1.0))
    (Transformation|SetWorldLocation (Variables|Default|GetCamera) (Math|Interpolation|VInterpTo _returnvalue (Variables|Movement|GetDesiredLocation) (Utilities|Time|GetWorldDeltaSeconds) (Variables|Movement|GetMovementLagSpeed)) false false)))

(fn InterpRotation
  (bind _camera (Variables|Default|GetCamera))
  (bind _returnvalue (Transformation|GetWorldRotation _camera))
  (if (not (Utilities|Operators|EqualEqual (Variables|Default|GetDesiredRotation) _returnvalue 1.0))
    (Transformation|SetWorldRotation (Variables|Default|GetCamera) (Math|Interpolation|RInterpTo _returnvalue (Variables|Default|GetDesiredRotation) (Utilities|Time|GetWorldDeltaSeconds) (Variables|Default|GetRotationLagSpeed)) false false)))

(fn UpdateMovementLagOffset
  (bind _maxmovementlagoffset (Variables|Movement|GetMaxMovementLagOffSet))
  (Variables|Movement|SetMovementLagOffset (Math|Interpolation|FInterpTo (Variables|Movement|GetMovementLagOffset) (Utilities|Select :Index (Variables|Movement|GetLagDirection) :Option%200 _maxmovementlagoffset :Option%201 _maxmovementlagoffset :Option%202 (* _maxmovementlagoffset 1.5)) (Utilities|Time|GetWorldDeltaSeconds) (Variables|Movement|GetMovementLagOffsetSpeed))))